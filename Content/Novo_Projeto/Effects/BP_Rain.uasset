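; BP_Rain is a weather actor that runs intermittent rain around the player.
; From BeginPlay it loops forever, switching the Chuva component on and off after random waits bounded by min/max variables for dry and rainy spells.
; Each spell spawns a rain sound at the player's current location and stops it shortly after the rain ends.
; Tick keeps Chuva at a fixed height above the player pawn.
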(event `self.ReceiveBeginPlay`
  (`ActorComponent.SetActive` (`self.Chuva`) false false :!label _label)
  (`KismetSystemLibrary.Delay` (`KismetMathLibrary.RandomFloatInRange` (`self.DelayMinimoChuva`) (`self.DelayMaximoChuva`)))
  (`ActorComponent.SetActive` (`self.Chuva`) true false)
  (`KismetSystemLibrary.Delay` 1.0)
  (bind _returnvalue (`GameplayStatics.SpawnSoundAtLocation` "/Game/Novo_Projeto/SFX/light-rain-109591.light-rain-109591" (`self.K2_GetActorLocation` (`GameplayStatics.GetPlayerPawn` 0)) (struct) 1.0 1.0 0.0 null null))
  (`KismetSystemLibrary.Delay` (`KismetMathLibrary.RandomFloatInRange` (`self.TempoMinimoChuva`) (`self.TempoMaximoChuva`)))
  (`ActorComponent.SetActive` (`self.Chuva`) false false)
  (`KismetSystemLibrary.Delay` 1.1)
  (`AudioComponent.Stop` _returnvalue)
  (goto _label))

(event `self.ReceiveTick`
  (params (DeltaSeconds :type "Float (single-precision)"))
  (`SceneComponent.K2_SetWorldLocation` (`self.Chuva`) (`KismetMathLibrary.MakeVector` (.x (`self.K2_GetActorLocation` (`GameplayStatics.GetPlayerPawn` 0))) (.y (`self.K2_GetActorLocation` (`GameplayStatics.GetPlayerPawn` 0))) (+ (.z (`self.K2_GetActorLocation` (`GameplayStatics.GetPlayerPawn` 0))) 700.0)) false false))

(fn `UserConstructionScript`)